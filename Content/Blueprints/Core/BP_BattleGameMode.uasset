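; Game mode for Zodie battles that switches control between the third-person player character and battling Zodie characters.
; BeginPlay spawns and possesses the player at BP_PlayerStart.
; StartBattle reads the active Zodie and enemy from BP_GameInstance, spawns both as BP_ZodieCharacter at their start markers via SpawnZodie, and possesses the player's Zodie.
; EndBattle repossesses the player and destroys both Zodies.
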(event `EndBattle`
  (`Controller.Possess` (`GameplayStatics.GetPlayerController` 0) (`self.Player`))
  (`self.K2_DestroyActor` (`self.Enemy Zodie`))
  (`self.K2_DestroyActor` (`self.Spawned Zodie`)))

(event `self.ReceiveBeginPlay`
  (bind _returnvalue (`GameplayStatics.GetActorOfClass` "/Game/Blueprints/Core/BP_PlayerStart.BP_PlayerStart_C"))
  (bind _returnvalue_2 (`|SpawnActorFromClass` "/Game/Blueprints/BP_ThirdPersonCharacter.BP_ThirdPersonCharacter_C" (`self.GetTransform` _returnvalue) "Undefined" "OverrideRootScale" null null))
  (bind _output_get (set `self.Player` _returnvalue_2))
  (`Controller.Possess` (`GameplayStatics.GetPlayerController` 0) _output_get))

(event `StartBattle`
  ;[1 1 1] get relevant data from game instance
  (bind _asbp_game_instance (cast `/Game/Blueprints/Core/BP_GameInstance` (`GameplayStatics.GetGameInstance`))
    (:`then`
      (bind _output_get (set `self.As BP Game Instance` _asbp_game_instance))
      (set `self.Active Zodie` (`/Game/Blueprints/Core/BP_GameInstance.ActiveZodie` _output_get))
      (set `self.Active Enemy` (`/Game/Blueprints/Core/BP_GameInstance.ActiveEnemy` _output_get))
      (`self.SpawnZodies`))
    (:`CastFailed`
      (`KismetSystemLibrary.PrintString` "Game Instance Bad"))))

(event `SpawnZodies`
  ;[1 1 1] Spawn Players Zodie
  (bind _returnvalue (`GameplayStatics.GetActorOfClass` "/Game/Blueprints/Core/BP_ZodieStart.BP_ZodieStart_C"))
  (bind _spawnedzodie (`self.SpawnZodie` _returnvalue (`self.Active Zodie`)))
  (bind _output_get (set `self.Spawned Zodie` _spawnedzodie))
  (`Controller.Possess` (`GameplayStatics.GetPlayerController` 0) _output_get)
  ;[1 1 1] Spawn Enemy Zodie
  (bind _returnvalue_2 (`GameplayStatics.GetActorOfClass` "/Game/Blueprints/Core/BP_EnemyStart.BP_EnemyStart_C"))
  (bind _spawnedzodie_2 (`self.SpawnZodie` _returnvalue_2 (`self.Active Enemy`)))
  (set `self.Enemy Zodie` _spawnedzodie_2))

(fn `SpawnZodie`
  (params (SpawnPoint :type "Actor Object Reference") (Zodie :type "/Game/Blueprints/Dev/Structs/Zodie_Struct Structure"))
  (returns (SpawnedZodie :type "Pawn Object Reference"))
  (bind _returnvalue (`|SpawnActorFromClass` "/Game/Blueprints/BP_ZodieCharacter.BP_ZodieCharacter_C" (`KismetMathLibrary.MakeTransform` (`self.K2_GetActorLocation` SpawnPoint) (`self.K2_GetActorRotation` SpawnPoint)) "Undefined" "OverrideRootScale" null null))
  (set `/Game/Blueprints/BP_ZodieCharacter.Zodie` Zodie _returnvalue)
  (return _returnvalue))

(fn `UserConstructionScript`)