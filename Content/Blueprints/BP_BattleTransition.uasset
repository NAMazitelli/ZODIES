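; BP_BattleTransition is a trigger actor that starts or ends a battle when something overlaps its Box component.
; On overlap, it casts the game mode to BP_BattleGameMode and calls StartBattle or EndBattle according to its StartBattle flag, with no check on the overlapping actor.
; BeginPlay copies the Text variable to a TextRender label, and a failed cast prints a debug string.
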(event `self.ReceiveBeginPlay`
  (`TextRenderComponent.K2_SetText` (`self.TextRender`) (`self.Text`)))

(event `self.Box.OnComponentBeginOverlap`
  (params (OverlappedComponent :type "PrimitiveComponent Object Reference") (OtherActor :type "Actor Object Reference") (OtherComp :type "PrimitiveComponent Object Reference") (OtherBodyIndex :type Integer) (bFromSweep :type Boolean) (SweepResult :type "HitResult Structure (by ref)"))
  (bind _asbp_battle_game_mode (cast `/Game/Blueprints/Core/BP_BattleGameMode` (`GameplayStatics.GetGameMode`))
    (:`then`
      (if (`self.StartBattle`)
        (`/Game/Blueprints/Core/BP_BattleGameMode.StartBattle` _asbp_battle_game_mode)
        (else
          (`/Game/Blueprints/Core/BP_BattleGameMode.EndBattle` _asbp_battle_game_mode))))
    (:`CastFailed`
      (`KismetSystemLibrary.PrintString` "FALLO"))))

(fn `UserConstructionScript`)