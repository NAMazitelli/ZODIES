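; BP_Partner is a companion character that follows the player around.
; On BeginPlay it caches the player as BP_ThirdPersonCharacter, printing a debug string if the cast fails, then starts FollowPlayer.
; FollowPlayer re-calls itself after a short delay, using AI MoveTo toward the player when at or beyond a distance threshold.
; When closer, it targets itself with the move, which halts it near the player.
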(event `self.ReceiveBeginPlay`
  (bind _asbp_third_person_character (cast `/Game/Blueprints/BP_ThirdPersonCharacter` (`GameplayStatics.GetPlayerCharacter` 0))
    (:`then`
      (set `self.As BP Third Person Character` _asbp_third_person_character)
      (`self.FollowPlayer`))
    (:`CastFailed`
      (`KismetSystemLibrary.PrintString` "malll"))))

(event `FollowPlayer`
  (if (>= (`self.GetDistanceTo` (`self.As BP Third Person Character`)) 200.0)
    (`|AIMoveTo` self (0.0 0.0 0.0) (`self.As BP Third Person Character`) 30.0
      (:`then`
        _))
    (else
      (`|AIMoveTo` self (0.0 0.0 0.0) self
        (:`then`
          _))))
  (`KismetSystemLibrary.Delay` 0.2)
  (`self.FollowPlayer`))

(fn `UserConstructionScript`)